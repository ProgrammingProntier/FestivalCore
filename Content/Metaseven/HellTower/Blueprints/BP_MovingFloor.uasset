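; BP_MovingFloor is a moving floor actor that either spins or slides its static mesh.
; After a start delay, MovingType selects one of four timelines: three drive a full yaw rotation, the fourth moves the mesh along relative X.
; The construction script applies MovingSpeed as the timelines' play rate and, when IsTwin is set, attaches a second mesh component to the main one so it follows the same motion.
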(event `self.ReceiveBeginPlay`
  (`KismetSystemLibrary.Delay` (`self.StartDelay`))
  (switch `int` (`self.MovingType`)
    (:`0`
      (bind (_direction _alpha) (`Timeline|MovingTimeline_0`)
        (:`Update`
          (`SceneComponent.K2_SetRelativeRotation` (`self.StaticMesh`) (`KismetMathLibrary.MakeRotator` 0.0 0.0 (`KismetMathLibrary.Lerp` 0.0 360.0 _alpha)) false false))))
    (:`1`
      (bind (_direction_2 _alpha_2) (`Timeline|MovingTimeline_1`)
        (:`Update`
          (`SceneComponent.K2_SetRelativeRotation` (`self.StaticMesh`) (`KismetMathLibrary.MakeRotator` 0.0 0.0 (`KismetMathLibrary.Lerp` 0.0 360.0 _alpha_2)) false false))))
    (:`2`
      (bind (_direction_3 _alpha_3) (`Timeline|MovingTimeline_2`)
        (:`Update`
          (`SceneComponent.K2_SetRelativeRotation` (`self.StaticMesh`) (`KismetMathLibrary.MakeRotator` 0.0 0.0 (`KismetMathLibrary.Lerp` 0.0 360.0 _alpha_3)) false false))))
    (:`3`
      (bind (_direction_4 _alpha_4) (`Timeline|MovingTimeline_3`)
        (:`Update`
          (`SceneComponent.K2_SetRelativeLocation` (`self.StaticMesh`) (`KismetMathLibrary.MakeVector` (`KismetMathLibrary.Lerp` 0.0 800.0 _alpha_4)) false false))))))

(fn `UserConstructionScript`
  (`TimelineComponent.SetPlayRate` (`self.MovingTimeline_0`) (`self.MovingSpeed`))
  (`TimelineComponent.SetPlayRate` (`self.MovingTimeline_1`) (`self.MovingSpeed`))
  (`TimelineComponent.SetPlayRate` (`self.MovingTimeline_2`) (`self.MovingSpeed`))
  (`TimelineComponent.SetPlayRate` (`self.MovingTimeline_3`) (`self.MovingSpeed`))
  (if (`self.bIsTwin`)
    (bind _returnvalue (`AddComponent|NODE_AddStaticMeshComponent-0` :`bManualAttachment` true))
    (`SceneComponent.K2_AttachToComponent` _returnvalue (`self.StaticMesh`) "None" "KeepRelative" "KeepRelative" "KeepRelative" true)))