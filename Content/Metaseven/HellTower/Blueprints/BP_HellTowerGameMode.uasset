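; Game mode for the Hell Tower minigame, which picks the highest player as winner when time runs out.
; On time-up it runs the parent logic, disables all player input, waits briefly, then shows the result through the festival game state.
; The winner comes from comparing each controlled pawn's world Z and keeping the player ID with the greatest height, reported as a single-winner set.
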(event `self.OnTimeIsUp`
  (`parent.OnTimeIsUp`)
  (`/Game/Core/Blueprints/Libraries/BP_FestivalFunctionLibrary.DisableAllPlayerInput`)
  (`KismetSystemLibrary.Delay` 2.0)
  (`/Game/Core/Blueprints/BP_FestivalGameState.ShowResult` (`self.GetFestivalGameState`) (`|MakeSet` (`self.CalculateWinnerID`)) false))

(fn `CalculateWinnerID`
  (returns (ReturnValue :type Integer))
  (locals (MaxPlayerZ :type "Float (double-precision)") (WinnerID :type Integer))
  (bind _controllerid (`/Game/Core/Blueprints/Libraries/BP_FestivalMacroLibrary.ForEachPlayer` self)
    (:`LoopBody`
      (bind (_returnvalue_x _returnvalue_y _returnvalue_z) (`KismetMathLibrary.BreakVector` (`self.K2_GetActorLocation` (`Controller.K2_GetPawn` (`GameplayStatics.GetPlayerControllerFromID` _controllerid)))))
      (if (> _returnvalue_z (`local.MaxPlayerZ`))
        (set `local.MaxPlayerZ` _returnvalue_z)
        (set `local.WinnerID` _controllerid)))
    (:`Completed`
      (return (`local.WinnerID`)))))

(fn `UserConstructionScript`
  (`parent.UserConstructionScript`))