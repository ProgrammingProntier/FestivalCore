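; Game mode for the ASMD festival minigame, a race to answer formulas correctly.
; On begin play it adds a spreadsheet widget to each player's screen, and the countdown's end reveals their formulas.
; Widget answer events add or subtract a point through the festival game state.
; The first player to ten wins, while running out of time shows a result with no winners.
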(event `self.ReceiveBeginPlay`
  (`parent.ReceiveBeginPlay`)
  (bind _controllerid (`/Game/Core/Blueprints/Libraries/BP_FestivalMacroLibrary.ForEachPlayer` self)
    (:`LoopBody`
      (bind _returnvalue (`|CreateWidget` "/Game/Metaseven/ASMD/Blueprints/WBP_Spreadsheet.WBP_Spreadsheet_C" (`GameplayStatics.GetPlayerControllerFromID` _controllerid)))
      (add `/Game/Metaseven/ASMD/Blueprints/WBP_Spreadsheet.OnAnswered` _returnvalue (delegate `AddScore`))
      (`KismetArrayLibrary.Array_Add` (`self.SpreadSheets`) _returnvalue)
      (`UserWidget.AddToPlayerScreen` _returnvalue 0))))

(event `AddScore`
  (params (bCorrect :type Boolean) (ControllerID :type Integer))
  (bind _returnvalue (`/Game/Core/Blueprints/BP_FestivalGameState.AddScore` (`self.GetFestivalGameState`) ControllerID (select `bool` bCorrect :`false` -1 :`true` 1)))
  (if (>= _returnvalue 10)
    (`/Game/Core/Blueprints/BP_FestivalGameState.ShowResult` (`self.GetFestivalGameState`) (`|MakeSet` ControllerID) true)))

(event `self.OnCountZero`
  (`parent.OnCountZero`)
  (`/Game/Metaseven/ASMD/Blueprints/WBP_Spreadsheet.ShowFormula` (`self.SpreadSheets`)))

(event `self.OnTimeIsUp`
  (`parent.OnTimeIsUp`)
  (`/Game/Core/Blueprints/BP_FestivalGameState.ShowResult` (`self.GetFestivalGameState`) (`|MakeSet`) true))

(fn `UserConstructionScript`
  (`parent.UserConstructionScript`))