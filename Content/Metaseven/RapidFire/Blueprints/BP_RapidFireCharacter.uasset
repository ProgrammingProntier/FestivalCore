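; Player character for the RapidFire game, scoring one point for its controller each time it uses an item.
; On BeginPlay it waits a tick, destroys itself if uncontrolled, otherwise caches the festival game state and binds AddScore to the use-item event.
; On possession it applies the player color for the controller ID to both the body and first-person meshes.
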(event `self.ReceiveBeginPlay`
  (`parent.ReceiveBeginPlay`)
  (`KismetSystemLibrary.DelayUntilNextTick`)
  (`/Engine/EditorBlueprintResources/StandardMacros.IsValid` (`self.GetController`)
    (:`Is Valid`
      (set `self.FestivalGameState` (`/Game/Core/Blueprints/Libraries/BP_FestivalFunctionLibrary.GetFestivalGameState`))
      (add `self.OnUseItem` (delegate `AddScore`)))
    (:`Is Not Valid`
      (`self.K2_DestroyActor`))))

(event `self.ReceivePossessed`
  (params (NewController :type "Controller Object Reference"))
  (`parent.ReceivePossessed` NewController)
  (`/Game/Core/Blueprints/Libraries/BP_FestivalFunctionLibrary.ApplyPlayerColor` (`self.Mesh`) (`self.GetControllerID`))
  (`/Game/Core/Blueprints/Libraries/BP_FestivalFunctionLibrary.ApplyPlayerColor` (`self.FirstPersonMesh`) (`self.GetControllerID`)))

(event `AddScore`
  (`/Game/Core/Blueprints/BP_FestivalGameState.AddScore` (`self.FestivalGameState`) (`self.GetControllerID`) 1))

(fn `UserConstructionScript`
  (`parent.UserConstructionScript`))