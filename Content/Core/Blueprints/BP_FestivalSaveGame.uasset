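; Festival save game that stores the gamepad-only option, a game filter and per-game play counts.
; Setters and play-count increments write the object straight to its save slot; both setters then fire change notifications.
; The gamepad-only setter also updates the project's skip-assigning-gamepad-to-player-1 map setting with the inverse value.
; Total plays are computed by summing the per-game count map.
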(fn `GetGameFilter`
  (returns (ReturnValue :type Integer))
  (return (`self.GameFilter`)))

(fn `GetPlayCount`
  (params (GameName :type String))
  (returns (ReturnValue :type Integer))
  (return (`BlueprintMapLibrary.Map_Find` (`self.PlayCounts`) GameName)))

(fn `GetTotalPlayCount`
  (returns (ReturnValue :type Integer))
  (locals (TotalPlayCount :type Integer))
  (bind _values (`BlueprintMapLibrary.Map_Values` (`self.PlayCounts`)))
  (for _array_element _values
    (set `local.TotalPlayCount` (+ (`local.TotalPlayCount`) _array_element)))
  (return (`local.TotalPlayCount`)))

(fn `GetUseGamepadOnly`
  (returns (ReturnValue :type Boolean))
  (return (`self.bUseGamepadOnly`)))

(fn `IncrementPlayCount`
  (params (GameName :type String))
  (`BlueprintMapLibrary.Map_Add` (`self.PlayCounts`) GameName (+ (`BlueprintMapLibrary.Map_Find` (`self.PlayCounts`) GameName) 1))
  (`GameplayStatics.SaveGameToSlot` self (`self.SlotName`))
  (return))

(fn `SetGameFilter`
  (params (NewValue :type Integer))
  (set `self.GameFilter` NewValue)
  (`GameplayStatics.SaveGameToSlot` self (`self.SlotName`))
  (`self.OnGameFilterChanged`)
  (return))

(fn `SetSkipAssigningGamepad`
  (`GameMapsSettings.SetSkipAssigningGamepadToPlayer1` (`GameMapsSettings.GetGameMapsSettings`) (not (`self.bUseGamepadOnly`)))
  (return))

(fn `SetUseGamepadOnly`
  (params (NewValue :type Boolean))
  (set `self.bUseGamepadOnly` NewValue)
  (`self.SetSkipAssigningGamepad`)
  (`GameplayStatics.SaveGameToSlot` self (`self.SlotName`))
  (`self.OnUseGamepadOnlyChanged`)
  (return))