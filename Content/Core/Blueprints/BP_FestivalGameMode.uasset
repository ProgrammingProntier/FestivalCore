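; Base game mode for Festival games, driving the match flow from a GameData asset: tutorial, ready, countdown, play and result.
; BeginPlay binds game state events, matches local player count to the game instance or a default, and sets splitscreen.
; Countdown widgets spawn per player in splitscreen, with only the last one triggering timer and music.
; Time-up and score-change handlers are empty hooks; showing results swaps music for a result sound.
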(event `self.ReceiveBeginPlay`
  (`self.GameData`
    (:`then`
      (`self.SetFestivalGameState`)
      (`self.AddPlayers`)
      (`GameplayStatics.SetForceDisableSplitscreen` (`/Game/Core/Blueprints/DataAssets/BP_GameData.bDisableSplitscreen` (`self.GameData`)))
      (if (`/Game/Core/Blueprints/DataAssets/BP_GameData.bShowTutorial` (`self.GameData`))
        (`self.ShowTutorial`)
        (else
          (`self.OnReady`))))
    (:`else`
      (`/Game/Core/Blueprints/Libraries/BP_PrintFunctionLibrary.PrintErrorString` (`KismetStringLibrary.Concat_StrStr` "Set " (`KismetSystemLibrary.GetDisplayName` self) ".GameData!")))))

(fn `AddPlayers`
  (locals (FestivalGameInstance :type "/Game/Core/Blueprints/BP_FestivalGameInstance Object Reference") (DesiredNumPlayers :type Integer :default 0) (MissingNumPlayers :type Integer))
  (set `local.FestivalGameInstance` (`/Game/Core/Blueprints/Libraries/BP_FestivalFunctionLibrary.GetFestivalGameInstance`))
  (set `local.DesiredNumPlayers` (`KismetMathLibrary.SelectInt` (`/Game/Core/Blueprints/BP_FestivalGameInstance.NumPlayers` (`local.FestivalGameInstance`)) (`/Game/Core/Blueprints/DataAssets/BP_GameData.DefaultNumPlayers` (`self.GameData`)) (`KismetMathLibrary.InRange_IntInt` (`/Game/Core/Blueprints/BP_FestivalGameInstance.NumPlayers` (`local.FestivalGameInstance`)) 1 4)))
  (bind _returnvalue (`self.GetNumPlayers`))
  (bind _output_get (set `local.MissingNumPlayers` (- (`local.DesiredNumPlayers`) _returnvalue)))
  (if (> _output_get 0)
    (for _ (range 1 (+ (`local.MissingNumPlayers`) 1))
      (`GameplayStatics.CreatePlayer` -1))
    (else
      (for _ (range (`local.MissingNumPlayers`) 0)
        (bind _returnvalue_2 (`self.GetNumPlayers`))
        (`GameplayStatics.RemovePlayer` (`GameplayStatics.GetPlayerControllerFromID` (- _returnvalue_2 1)) true))))
  (return))

(fn `GetFestivalGameState`
  (returns (ReturnValue :type "/Game/Core/Blueprints/BP_FestivalGameState Object Reference"))
  (return (`self.FestivalGameState`)))

(fn `OnCountZero`
  (`/Game/Core/Blueprints/BP_FestivalGameState.StartTimer` (`self.FestivalGameState`))
  (`/Game/Core/Blueprints/BP_FestivalGameState.LoadAndPlayMusic` (`self.FestivalGameState`) (`/Game/Core/Blueprints/DataAssets/BP_AudioData.GameMusic` (`/Game/Core/Blueprints/DataAssets/BP_GameData.AudioData` (`self.GameData`))))
  (`/Game/Core/Blueprints/BP_FestivalGameState.OnCountZero` (`self.FestivalGameState`))
  (return))

(fn `OnReady`
  (bind _timelimit (`/Game/Core/Blueprints/DataAssets/BP_GameData.TimeLimit` (`self.GameData`)))
  (`|ExecutionSequence`
    (:`then_0`
      (if (> _timelimit 0)
        (`/Game/Core/Blueprints/BP_FestivalGameState.SetTimer` (`self.FestivalGameState`) _timelimit)))
    (:`then_1`
      (if (`/Game/Core/Blueprints/DataAssets/BP_GameData.bShowScore` (`self.GameData`))
        (`/Game/Core/Blueprints/BP_FestivalGameState.ShowScore` (`self.FestivalGameState`))))
    (:`then_2`
      (if (`/Game/Core/Blueprints/DataAssets/BP_GameData.bShowCountdown` (`self.GameData`))
        (`self.ShowCountdown`)
        (else
          (`self.OnCountZero`))))
    (:`then_3`
      (`/Game/Core/Blueprints/BP_FestivalGameState.OnReady` (`self.FestivalGameState`))
      (return))))

(fn `OnScoreChanged`
  (params (ControllerID :type Integer) (Score :type Integer))
  (return))

(fn `OnShowResult`
  (`/Game/Core/Blueprints/BP_FestivalGameState.ClearTimer` (`self.FestivalGameState`) 4.0)
  (`AudioComponent.Stop` (`/Game/Core/Blueprints/BP_FestivalGameState.MusicAudio` (`self.FestivalGameState`)))
  (`/Game/Core/Blueprints/BP_FestivalGameState.LoadAndPlaySound` (`self.FestivalGameState`) (`/Game/Core/Blueprints/DataAssets/BP_AudioData.ResultSound` (`/Game/Core/Blueprints/DataAssets/BP_GameData.AudioData` (`self.GameData`))))
  (return))

(fn `OnTimeIsUp`
  (return))

(fn `SetFestivalGameState`
  (set `self.FestivalGameState` (`/Game/Core/Blueprints/Libraries/BP_FestivalFunctionLibrary.GetFestivalGameState`))
  (add `/Game/Core/Blueprints/BP_FestivalGameState.OnShowResult` (`self.FestivalGameState`) (`|CreateDelegate` :!event `OnShowResult`))
  (add `/Game/Core/Blueprints/BP_FestivalGameState.OnTimeIsUp` (`self.FestivalGameState`) (`|CreateDelegate` :!event `OnTimeIsUp`))
  (add `/Game/Core/Blueprints/BP_FestivalGameState.OnScoreChanged` (`self.FestivalGameState`) (`|CreateDelegate` :!event `OnScoreChanged`))
  (return))

(fn `ShowCountdown`
  (locals (CountdownWidget :type "/Game/Core/Blueprints/UI/WBP_Countdown Object Reference"))
  (if (`GameplayStatics.IsSplitscreenForceDisabled`)
    (bind _returnvalue (`|CreateWidget` "/Game/Core/Blueprints/UI/WBP_Countdown.WBP_Countdown_C" null (`/Game/Core/Blueprints/DataAssets/BP_GameData.AudioData` (`self.GameData`))))
    (bind _output_get (set `local.CountdownWidget` _returnvalue))
    (`UserWidget.AddToViewport` _output_get 1)
    (add `/Game/Core/Blueprints/UI/WBP_Countdown.OnCountZero` (`local.CountdownWidget`) (`|CreateDelegate` :!event `OnCountZero`) :!label _label)
    (return)
    (else
      (bind _controllerid (`/Game/Core/Blueprints/Libraries/BP_FestivalMacroLibrary.ForEachPlayer` self)
        (:`LoopBody`
          (bind _returnvalue_2 (`|CreateWidget` "/Game/Core/Blueprints/UI/WBP_Countdown.WBP_Countdown_C" (`GameplayStatics.GetPlayerControllerFromID` _controllerid) (`/Game/Core/Blueprints/DataAssets/BP_GameData.AudioData` (`self.GameData`))))
          (bind _output_get_2 (set `local.CountdownWidget` _returnvalue_2))
          (`UserWidget.AddToPlayerScreen` _output_get_2 1))
        (:`Completed`
          (goto _label))))))

(fn `ShowTutorial`
  (bind _returnvalue (`|CreateWidget` "/Game/Core/Blueprints/UI/WBP_Tutorial.WBP_Tutorial_C" null (`self.GameData`)))
  (add `/Game/Core/Blueprints/UI/WBP_Tutorial.OnReady` _returnvalue (`|CreateDelegate` :!event `OnReady`))
  (`UserWidget.AddToViewport` _returnvalue 1)
  (`/Game/Core/Blueprints/BP_FestivalGameState.LoadAndPlayMusic` (`self.FestivalGameState`) (`/Game/Core/Blueprints/DataAssets/BP_AudioData.TutorialMusic` (`/Game/Core/Blueprints/DataAssets/BP_GameData.AudioData` (`self.GameData`))))
  (return))

(fn `UserConstructionScript`)