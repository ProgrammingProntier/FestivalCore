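; Blueprint function library of shared helpers for the Festival game, covering typed access to its game instance and game state, local player utilities and player colors.
; A ForEachPlayer loop enables or disables input on every valid controlled pawn and collects the IDs of players with pawns.
; Controller IDs are range-checked against the local controller count.
; Each ID maps to a palette accent color, applied to mesh tint and logo layer material parameters.
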(fn `ApplyPlayerColor`
  (params (Mesh :type "MeshComponent Object Reference") (ControllerID :type Integer))
  (locals (Color :type "Vector Structure"))
  (set `local.Color` (`KismetMathLibrary.Conv_LinearColorToVector` (`self.GetPlayerColor` ControllerID)))
  (`MeshComponent.SetVectorParameterValueOnMaterials` Mesh "Tint" (`local.Color`))
  (`MeshComponent.SetVectorParameterValueOnMaterials` Mesh "LogoLayer0_Color" (`local.Color`))
  (`MeshComponent.SetVectorParameterValueOnMaterials` Mesh "LogoLayer1_Color" (`local.Color`))
  (`MeshComponent.SetVectorParameterValueOnMaterials` Mesh "LogoLayer2_Color" (`local.Color`))
  (return))

(fn `DisableAllPlayerInput`
  (bind _controllerid (`/Game/Core/Blueprints/Libraries/BP_FestivalMacroLibrary.ForEachPlayer` (`GameplayStatics.GetGameMode` null))
    (:`LoopBody`
      (bind _returnvalue (`Controller.K2_GetPawn` (`GameplayStatics.GetPlayerControllerFromID` null _controllerid)))
      (`/Engine/EditorBlueprintResources/StandardMacros.IsValid` _returnvalue
        (:`Is Valid`
          (`Actor.DisableInput` _returnvalue null))))
    (:`Completed`
      (return))))

(fn `EnableAllPlayerInput`
  (bind _controllerid (`/Game/Core/Blueprints/Libraries/BP_FestivalMacroLibrary.ForEachPlayer` (`GameplayStatics.GetGameMode` null))
    (:`LoopBody`
      (bind _returnvalue (`Controller.K2_GetPawn` (`GameplayStatics.GetPlayerControllerFromID` null _controllerid)))
      (`/Engine/EditorBlueprintResources/StandardMacros.IsValid` _returnvalue
        (:`Is Valid`
          (`Actor.EnableInput` _returnvalue null))))
    (:`Completed`
      (return))))

(fn `GetFestivalGameInstance`
  (returns (ReturnValue :type "/Game/Core/Blueprints/BP_FestivalGameInstance Object Reference"))
  (return (cast `/Game/Core/Blueprints/BP_FestivalGameInstance` (`GameplayStatics.GetGameInstance` null) :!pure true)))

(fn `GetFestivalGameState`
  (returns (ReturnValue :type "/Game/Core/Blueprints/BP_FestivalGameState Object Reference"))
  (return (cast `/Game/Core/Blueprints/BP_FestivalGameState` (`GameplayStatics.GetGameState` null) :!pure true)))

(fn `GetPlayerColor`
  (params (ControllerID :type Integer))
  (returns (ReturnValue :type "LinearColor Structure"))
  (locals (PaletteData :type "/Game/Core/Blueprints/DataAssets/BP_PaletteData Object Reference" :default "BP_PaletteData_C'/Game/Core/Data/DA_DefaultPalette.DA_DefaultPalette'"))
  (return (`/Game/Core/Blueprints/DataAssets/BP_PaletteData.GetAccentColor` (`local.PaletteData`) ControllerID)))

(fn `GetValidPlayerIDs`
  (returns (ReturnValue :type "Array of Integer"))
  (locals (ValidPlayerIDs :type "Array of Integer"))
  (bind _controllerid (`/Game/Core/Blueprints/Libraries/BP_FestivalMacroLibrary.ForEachPlayer` (`GameplayStatics.GetGameMode` null))
    (:`LoopBody`
      (`/Engine/EditorBlueprintResources/StandardMacros.IsValid` (`Controller.K2_GetPawn` (`GameplayStatics.GetPlayerControllerFromID` null _controllerid))
        (:`Is Valid`
          (`KismetArrayLibrary.Array_Add` (`local.ValidPlayerIDs`) _controllerid))))
    (:`Completed`
      (return (`local.ValidPlayerIDs`)))))

(fn `IsValidControllerID`
  (params (ControllerID :type Integer))
  (returns (ReturnValue :type Boolean))
  (return (`KismetMathLibrary.InRange_IntInt` ControllerID 0 (`GameplayStatics.GetNumLocalPlayerControllers` null) true false)))