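; Game mode for the game selection screen, which sets up the menu and its music when play begins.
; On BeginPlay it removes every player after the first, destroying their pawns.
; If GameSelectData is valid, it creates the WBP_GameSelect widget with that asset's game list, adds it to the viewport and plays the asset's music through the MusicAudio component.
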(event `self.ReceiveBeginPlay`
  (`self.RemovePlayers`)
  (`self.ShowWidget`))

(fn `RemovePlayers`
  (bind _returnvalue (`self.GetNumPlayers`))
  (for _index (range 1 _returnvalue)
    (`GameplayStatics.RemovePlayer` (`GameplayStatics.GetPlayerControllerFromID` _index) true))
  (return))

(fn `ShowWidget`
  (bind _gameselectdata (`self.GameSelectData`)
    (:`then`
      (bind _returnvalue (`|CreateWidget` "/Game/Core/Blueprints/GameSelect/WBP_GameSelect.WBP_GameSelect_C" null (`/Game/Core/Blueprints/GameSelect/BP_GameSelectData.AllGameData` _gameselectdata)))
      (`UserWidget.AddToViewport` _returnvalue 0)
      (`AudioComponent.SetSound` (`self.MusicAudio`) (`/Game/Core/Blueprints/GameSelect/BP_GameSelectData.Music` (`self.GameSelectData`)))
      (`AudioComponent.Play` (`self.MusicAudio`) 0.0)
      (return))
    (:`else`
      (return))))

(fn `UserConstructionScript`)