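; Player controller for the game select stage that lets the player toggle the settings menu.
; On possess it sets game-only input and adds the menu-open Enhanced Input mapping context.
; When the menu action completes, it calls MenuReturn if WBP_Settings is the active UINav widget.
; Otherwise it creates a new settings widget and navigates to it through the active widget, keeping the parent.
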(event `self.ReceivePossess`
  (params (PossessedPawn :type "Pawn Object Reference"))
  (`parent.ReceivePossess` PossessedPawn)
  (`WidgetBlueprintLibrary.SetInputMode_GameOnly` self)
  (`EnhancedInputSubsystemInterface.AddMappingContext` (subsystem `EnhancedInputLocalPlayerSubsystem`) "/Game/Core/Inputs/IC_MenuOpen.IC_MenuOpen" 0 (struct)))

(event `EnhancedInput|/Game/Core/Inputs/IA_MenuOpen`
  (params (ActionValue :type Boolean) (ElapsedSeconds :type "Float (double-precision)") (TriggeredSeconds :type "Float (double-precision)") (InputAction :type "InputAction Object Reference" :default "/Game/Core/Inputs/IA_MenuOpen.IA_MenuOpen"))
  (:`Completed`
    (if (== (`GameplayStatics.GetObjectClass` (`UINavPCComponent.GetActiveWidget` (`self.UINavPCComp`))) "/Game/Core/Blueprints/GameSelect/WBP_Settings.WBP_Settings_C")
      (`UINavWidget.MenuReturn` (`UINavPCComponent.GetActiveWidget` (`self.UINavPCComp`)))
      (else
        (bind _returnvalue (`|CreateWidget` "/Game/Core/Blueprints/GameSelect/WBP_Settings.WBP_Settings_C" self))
        (`UINavWidget.GoToBuiltWidget` (`UINavPCComponent.GetActiveWidget` (`self.UINavPCComp`)) _returnvalue false false 0)))))

(fn `UserConstructionScript`
  (`parent.UserConstructionScript`))