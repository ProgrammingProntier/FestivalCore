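; BP_IconData is an icon data asset that maps input keys to their icons for keyboard, Xbox One and PS4.
; Each platform has its own map, read by a matching getter that takes a key and returns the found value.
; The getters ignore whether the key was found and have no fallback between platforms.
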(fn `GetKeyboardIcon`
  (params (Key :type "Key Structure" :default "None"))
  (returns (ReturnValue :type "Texture2D Soft Object Reference"))
  (return (`BlueprintMapLibrary.Map_Find` (`self.KeyboardIcons`) Key)))

(fn `GetPS4Icon`
  (params (Key :type "Key Structure" :default "None"))
  (returns (ReturnValue :type "Texture2D Soft Object Reference"))
  (return (`BlueprintMapLibrary.Map_Find` (`self.PS4Icons`) Key)))

(fn `GetXboxOneIcon`
  (params (Key :type "Key Structure" :default "None"))
  (returns (ReturnValue :type "Texture2D Soft Object Reference"))
  (return (`BlueprintMapLibrary.Map_Find` (`self.XboxOneIcons`) Key)))