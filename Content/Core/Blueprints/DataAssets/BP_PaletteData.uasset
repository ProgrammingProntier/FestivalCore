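; BP_PaletteData is a palette data asset that stores text, background and accent colors.
; Each color role has its own array, read through a getter that takes an index.
; The getters return the array element directly, with no bounds check or fallback color.
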(fn `GetAccentColor`
  (params (Index :type Integer))
  (returns (ReturnValue :type "LinearColor Structure"))
  (return (`|GetArrayItem` (`self.AccentColors`) Index)))

(fn `GetBackgroundColor`
  (params (Index :type Integer))
  (returns (ReturnValue :type "LinearColor Structure"))
  (return (`|GetArrayItem` (`self.BackgroundColors`) Index)))

(fn `GetTextColor`
  (params (Index :type Integer))
  (returns (ReturnValue :type "LinearColor Structure"))
  (return (`|GetArrayItem` (`self.TextColors`) Index)))