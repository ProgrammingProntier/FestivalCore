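; BP_GameData is a game data asset whose functions query and format which player counts, one to four, a game allows.
; IsAllowedNumPlayers maps a count to its AllowedNumPlayers flag, with zero always allowed.
; GetAllowedNumPlayersString concatenates the enabled counts and compacts them into range notation using "~" and "," separators.
; GetAllowedNumPlayersTexts returns a Japanese "人" label for each enabled count.
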(fn `GetAllowedNumPlayersString`
  (returns (ReturnValue :type String))
  (locals (SourceString :type String) (LeftS :type String) (RightS :type String))
  (bind _sourcestring (`local.SourceString`))
  (bind _rights (`local.RightS`))
  (bind _lefts (`local.LeftS`))
  (bind (_lefts_2 _rights_2) (`KismetStringLibrary.Split` (`local.SourceString`) " "))
  (set `local.SourceString` (`KismetStringLibrary.TrimTrailing` (`KismetStringLibrary.Trim` (`KismetStringLibrary.Concat_StrStr` (`KismetMathLibrary.SelectString` "1" " " (`.1P_8_5760111845596FFD3DB13F9FD27B2A82` (break `/Game/Core/Data/S_AllowedNumPlayers` (`self.AllowedNumPlayers`)))) (`KismetMathLibrary.SelectString` "2" " " (`.2P_9_A626EB9F46EFBDE0A61ED786B40D12AF` (break `/Game/Core/Data/S_AllowedNumPlayers` (`self.AllowedNumPlayers`)))) (`KismetMathLibrary.SelectString` "3" " " (`.3P_10_F133D6FD45C9B08549C55886CA392B70` (break `/Game/Core/Data/S_AllowedNumPlayers` (`self.AllowedNumPlayers`)))) (`KismetMathLibrary.SelectString` "4" " " (`.4P_7_24B88E9148F2979E58F9638BA2863A6C` (break `/Game/Core/Data/S_AllowedNumPlayers` (`self.AllowedNumPlayers`))))))))
  (`|ExecutionSequence`
    (:`then_0`
      (if (`KismetStringLibrary.Contains` (`local.SourceString`) " ")
        (set `local.LeftS` _lefts_2)
        (set `local.RightS` (`KismetStringLibrary.Trim` _rights_2))
        (`|ExecutionSequence`
          (:`then_0`
            (if (> (`KismetStringLibrary.Len` (`local.LeftS`)) 1)
              (set `local.LeftS` (`KismetStringLibrary.Concat_StrStr` (`KismetStringLibrary.Left` _lefts 1) "~" (`KismetStringLibrary.Right` _lefts 1)))
              (elif (> (`KismetStringLibrary.Len` (`local.RightS`)) 1)
                (set `local.RightS` (`KismetStringLibrary.Concat_StrStr` (`KismetStringLibrary.Left` _rights 1) "~" (`KismetStringLibrary.Right` _rights 1))))))
          (:`then_1`
            (set `local.SourceString` (`KismetStringLibrary.Concat_StrStr` (`local.LeftS`) "," (`local.RightS`)))))
        (elif (> (`KismetStringLibrary.Len` (`local.SourceString`)) 1)
          (set `local.SourceString` (`KismetStringLibrary.Concat_StrStr` (`KismetStringLibrary.Left` _sourcestring 1) "~" (`KismetStringLibrary.Right` _sourcestring 1))))))
    (:`then_1`
      (return (`local.SourceString`)))))

(fn `GetAllowedNumPlayersTexts`
  (returns (ReturnValue :type "Array of Text"))
  (locals (Texts :type "Array of Text"))
  (`|ExecutionSequence`
    (:`then_0`
      (if (`.1P_8_5760111845596FFD3DB13F9FD27B2A82` (break `/Game/Core/Data/S_AllowedNumPlayers` (`self.AllowedNumPlayers`)))
        (`KismetArrayLibrary.Array_Add` (`local.Texts`) "1人")))
    (:`then_1`
      (if (`.2P_9_A626EB9F46EFBDE0A61ED786B40D12AF` (break `/Game/Core/Data/S_AllowedNumPlayers` (`self.AllowedNumPlayers`)))
        (`KismetArrayLibrary.Array_Add` (`local.Texts`) "2人")))
    (:`then_2`
      (if (`.3P_10_F133D6FD45C9B08549C55886CA392B70` (break `/Game/Core/Data/S_AllowedNumPlayers` (`self.AllowedNumPlayers`)))
        (`KismetArrayLibrary.Array_Add` (`local.Texts`) "3人")))
    (:`then_3`
      (if (`.4P_7_24B88E9148F2979E58F9638BA2863A6C` (break `/Game/Core/Data/S_AllowedNumPlayers` (`self.AllowedNumPlayers`)))
        (`KismetArrayLibrary.Array_Add` (`local.Texts`) "4人")))
    (:`then_4`
      (return (`local.Texts`)))))

(fn `IsAllowedNumPlayers`
  (params (NumPlayers :type Integer))
  (returns (ReturnValue :type Boolean))
  (bind (_allowednumplayers_1p _allowednumplayers_2p _allowednumplayers_3p _allowednumplayers_4p) (break `/Game/Core/Data/S_AllowedNumPlayers` (`self.AllowedNumPlayers`)))
  (return (select `int` NumPlayers :`0` true :`1` _allowednumplayers_1p :`2` _allowednumplayers_2p :`3` _allowednumplayers_3p :`4` _allowednumplayers_4p)))