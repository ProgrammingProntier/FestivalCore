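; Player controller for the Festival game that sets up input on possession and handles the quit menu and debug shortcuts.
; Possession activates the UINav component, sets game-only input, and adds the menu-open mapping context above a configurable context list, warning if that list is empty.
; The menu action creates WBP_QuitGame or calls MenuReturn on an existing one.
; Hard-wired keys restart the level, toggle pause and toggle slow motion.
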(event Input|EnhancedActionEvents|EnhancedInputActionIA_MenuOpen
  (params (ActionValue :type Boolean) (ElapsedSeconds :type Float%20%28double-precision%29) (TriggeredSeconds :type Float%20%28double-precision%29) (InputAction :type Input%20Action%20Object%20Reference :default "/Game/Core/Inputs/IA_MenuOpen.IA_MenuOpen"))
  (:Completed
    (bind _foundwidgets (Widget|GetAllWidgetsOfClass "/Game/Core/Blueprints/UI/WBP_QuitGame.WBP_QuitGame_C" true))
    (if (Utilities|Array|IsEmpty _foundwidgets)
      (bind _returnvalue (UserInterface|CreateWidget "/Game/Core/Blueprints/UI/WBP_QuitGame.WBP_QuitGame_C" self))
      (UserInterface|Viewport|AddtoViewport _returnvalue 1)
      (else
        (Class|UINavWidget|MenuReturn (Utilities|Array|Get(acopy) _foundwidgets))))))

(event EventPossess
  (params (PossessedPawn :type Pawn%20Object%20Reference))
  (|CallParentFunction PossessedPawn)
  (Components|Activation|Activate (Variables|Default|GetUINavPCComp) false)
  (Input|SetInputModeGameOnly self)
  (Input|AddMappingContext (PlayerController|LocalPlayerSubsystems|GetEnhancedInputLocalPlayerSubsystem) "/Game/Core/Inputs/IC_MenuOpen.IC_MenuOpen" 1 "(bIgnoreAllPressedKeysUntilRelease=True,bForceImmediately=False)")
  (if (Utilities|Array|IsNotEmpty (Variables|Festival|GetMappingContexts))
    (for _array_element (Variables|Festival|GetMappingContexts)
      (Input|AddMappingContext (PlayerController|LocalPlayerSubsystems|GetEnhancedInputLocalPlayerSubsystem) _array_element 0 "(bIgnoreAllPressedKeysUntilRelease=True,bForceImmediately=False)"))
    (else
      (CallFunction|PrintWarningString (Utilities|String|Append "Set " (Utilities|GetDisplayName self) ".MappingContexts!")))))

(event Input|KeyboardEvents|DebugKeyZ
  (params (Key :type Key%20Structure :default "None") (ActionValue :type Input%20Action%20Value%20Structure))
  (:Pressed
    (if (== (Class|GameplayStatics|GetGlobalTimeDilation) 1.0)
      (Utilities|Time|SetGlobalTimeDilation 0.1)
      (else
        (Utilities|Time|SetGlobalTimeDilation 1.0)))))

(event Input|KeyboardEvents|DebugKeyX
  (params (Key :type Key%20Structure :default "None") (ActionValue :type Input%20Action%20Value%20Structure))
  (:Pressed
    (Game|SetGamePaused (not (Game|IsGamePaused)))))

(event Input|KeyboardEvents|R
  (params (Key :type Key%20Structure :default "None"))
  (:Pressed
    (Development|ExecuteConsoleCommand "RestartLevel" 0)))

(fn ConstructionScript)