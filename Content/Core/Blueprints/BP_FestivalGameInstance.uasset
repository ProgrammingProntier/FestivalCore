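; Game instance that owns the festival save game object for the session.
; On Init it loads the save from the configured slot, or creates a new one if none exists or the loaded object fails to cast.
; It then calls SetSkipAssigningGamepad on the save and exposes it through a getter.
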(event `self.ReceiveInit`
  (`self.InitSaveGame`))

(fn `GetFestivalSaveGame`
  (returns (ReturnValue :type "/Game/Core/Blueprints/BP_FestivalSaveGame Object Reference"))
  (return (`self.FestivalSaveGame`)))

(fn `InitSaveGame`
  (locals (SlotName :type String :default "FestivalSaveGame"))
  (bind _returnvalue (`GameplayStatics.DoesSaveGameExist` (`local.SlotName`)))
  (if _returnvalue
    (bind _returnvalue_2 (`GameplayStatics.LoadGameFromSlot` (`local.SlotName`)))
    (bind _asbp_festival_save_game (cast `/Game/Core/Blueprints/BP_FestivalSaveGame` _returnvalue_2)
      (:`then`
        (set `self.FestivalSaveGame` _asbp_festival_save_game))
      (:`CastFailed`
        (bind _returnvalue_3 (`GameplayStatics.CreateSaveGameObject` "/Game/Core/Blueprints/BP_FestivalSaveGame.BP_FestivalSaveGame_C" :!label _label))
        (set `self.FestivalSaveGame` _returnvalue_3)))
    (else
      (goto _label)))
  (`/Game/Core/Blueprints/BP_FestivalSaveGame.SetSkipAssigningGamepad` (`self.FestivalSaveGame`))
  (return))