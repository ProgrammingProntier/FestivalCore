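; Festival game state that provides a shared timer, per-player scores, win/lose/draw results and audio playback for local players.
; Timer and score functions delegate to lazily created widgets, whose time-up and score-change events it relays.
; Score and result widgets go on each player's screen, or on the viewport when splitscreen is force-disabled.
; Sounds and music async-load from soft references, with music playing through a MusicAudio component.
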(event `LoadAndPlaySound`
  (params (Sound :type "Object Soft Object Reference"))
  (if (`KismetSystemLibrary.IsValidSoftObjectReference` Sound)
    (bind _object (`|LoadAsset` Sound)
      (:`Completed`
        (`GameplayStatics.PlaySoundAtLocation` (cast `SoundBase` _object :!pure true) (0.0 0.0 0.0) (struct) 1.0 1.0 0.0 null null null null)))))

(event `LoadAndPlayMusic`
  (params (Music :type "SoundBase Soft Object Reference"))
  (if (`KismetSystemLibrary.IsValidSoftObjectReference` Music)
    (bind _object (`|LoadAsset` Music)
      (:`Completed`
        (`AudioComponent.SetSound` (`self.MusicAudio`) (cast `SoundBase` _object :!pure true))
        (`AudioComponent.Play` (`self.MusicAudio`) 0.0)))))

(fn `AddScore`
  (params (ControllerID :type Integer) (Score :type Integer))
  (returns (ReturnValue :type Integer))
  (if (`KismetArrayLibrary.Array_IsValidIndex` (`self.ScoreWidgets`) ControllerID)
    (bind _returnvalue (`/Game/Core/Blueprints/UI/WBP_Score.AddScore` (`|GetArrayItem` (`self.ScoreWidgets`) ControllerID) Score))
    (return _returnvalue)
    (else
      (return 0))))

(fn `AddTime`
  (params (Time :type "Float (double-precision)"))
  (returns (ReturnValue :type "Float (double-precision)"))
  (bind _timerwidget (`self.TimerWidget`)
    (:`then`
      (bind _returnvalue (`/Game/Core/Blueprints/UI/WBP_Timer.AddTime` _timerwidget Time))
      (return _returnvalue))
    (:`else`
      (return 0.0))))

(fn `CallOnScoreChanged`
  (params (ControllerID :type Integer) (Score :type Integer))
  (`self.OnScoreChanged` ControllerID Score)
  (return))

(fn `CallOnTimeIsUp`
  (`self.OnTimeIsUp`)
  (return))

(fn `ClearTimer`
  (params (TimeToRemove :type "Float (single-precision)"))
  (bind _timerwidget (`self.TimerWidget`)
    (:`then`
      (`/Game/Core/Blueprints/UI/WBP_Timer.ClearTimer` _timerwidget TimeToRemove)
      (set `self.TimerWidget` null)
      (return))
    (:`else`
      (return))))

(fn `GetMaxScore`
  (returns (MaxScoreIDs :type "Set of Integer") (ReturnValue :type Integer))
  (locals (MaxScore :type Integer :default -2147483648) (MaxScoreIndexes :type "Set of Integer"))
  (for (_array_element _array_index) (`self.ScoreWidgets`)
    (bind _returnvalue (`/Game/Core/Blueprints/UI/WBP_Score.GetScore` _array_element))
    (`/Engine/EditorBlueprintResources/StandardMacros.CompareInt` _returnvalue (`local.MaxScore`)
      (:`>`
        (set `local.MaxScore` _returnvalue)
        (`BlueprintSetLibrary.Set_Clear` (`local.MaxScoreIndexes`)))
      (:`==`
        _))
    (`BlueprintSetLibrary.Set_Add` (`local.MaxScoreIndexes`) _array_index))
  (return (`local.MaxScoreIndexes`) (`local.MaxScore`)))

(fn `GetMinScore`
  (returns (MinScoreIDs :type "Set of Integer") (ReturnValue :type Integer))
  (locals (MinScore :type Integer :default 2147483647) (MinScoreIndexes :type "Set of Integer"))
  (for (_array_element _array_index) (`self.ScoreWidgets`)
    (bind _returnvalue (`/Game/Core/Blueprints/UI/WBP_Score.GetScore` _array_element))
    (`/Engine/EditorBlueprintResources/StandardMacros.CompareInt` _returnvalue (`local.MinScore`)
      (:`==`
        _)
      (:`<`
        (set `local.MinScore` _returnvalue)
        (`BlueprintSetLibrary.Set_Clear` (`local.MinScoreIndexes`))))
    (`BlueprintSetLibrary.Set_Add` (`local.MinScoreIndexes`) _array_index))
  (return (`local.MinScoreIndexes`) (`local.MinScore`)))

(fn `GetScore`
  (params (ControllerID :type Integer))
  (returns (ReturnValue :type Integer))
  (if (`KismetArrayLibrary.Array_IsValidIndex` (`self.ScoreWidgets`) ControllerID)
    (return (`/Game/Core/Blueprints/UI/WBP_Score.GetScore` (`|GetArrayItem` (`self.ScoreWidgets`) ControllerID)))
    (else
      (return 0))))

(fn `GetTime`
  (returns (ReturnValue :type "Float (double-precision)"))
  (bind _timerwidget (`self.TimerWidget`)
    (:`then`
      (return (`/Game/Core/Blueprints/UI/WBP_Timer.GetTime` _timerwidget)))
    (:`else`
      (return 0.0))))

(fn `HideScore`
  (`/Game/Core/Blueprints/UI/WBP_Score.HideScore` (`self.ScoreWidgets`))
  (return))

(fn `HideTimer`
  (bind _timerwidget (`self.TimerWidget`)
    (:`then`
      (`/Game/Core/Blueprints/UI/WBP_Timer.HideTimer` _timerwidget)
      (return))
    (:`else`
      (return))))

(fn `ResetScore`
  (`/Game/Core/Blueprints/UI/WBP_Score.ResetScore` (`self.ScoreWidgets`))
  (return))

(fn `SetScore`
  (params (ControllerID :type Integer) (Score :type Integer))
  (returns (ReturnValue :type Integer))
  (if (`KismetArrayLibrary.Array_IsValidIndex` (`self.ScoreWidgets`) ControllerID)
    (bind _returnvalue (`/Game/Core/Blueprints/UI/WBP_Score.SetScore` (`|GetArrayItem` (`self.ScoreWidgets`) ControllerID) Score))
    (return _returnvalue)
    (else
      (return 0))))

(fn `SetTimer`
  (params (Time :type Integer))
  (`self.TimerWidget`
    (:`then`
      _)
    (:`else`
      (bind _returnvalue (`|CreateWidget` "/Game/Core/Blueprints/UI/WBP_Timer.WBP_Timer_C"))
      (bind _output_get (set `self.TimerWidget` _returnvalue))
      (add `/Game/Core/Blueprints/UI/WBP_Timer.OnTimeIsUp` _output_get (`|CreateDelegate` :!event `CallOnTimeIsUp`))
      (`UserWidget.AddToViewport` (`self.TimerWidget`) 1)))
  (`/Game/Core/Blueprints/UI/WBP_Timer.SetTimer` (`self.TimerWidget`) Time)
  (return))

(fn `ShowResult`
  (params (WinnerIDs :type "Set of Integer") (DisableInput :type Boolean))
  (if (not (`self.bShowResult`))
    (set `self.bShowResult` true)
    (`self.OnShowResult`)
    (if (`local.DisableInput`)
      (`/Game/Core/Blueprints/Libraries/BP_FestivalFunctionLibrary.DisableAllPlayerInput`))
    (bind _result (`BlueprintSetLibrary.Set_ToArray` (`local.WinnerIDs`)))
    (for _array_element _result
      (if (not (`/Game/Core/Blueprints/Libraries/BP_FestivalFunctionLibrary.IsValidControllerID` _array_element))
        (`BlueprintSetLibrary.Set_Remove` (`local.WinnerIDs`) _array_element)))
    (if (> (`GameplayStatics.GetNumLocalPlayerControllers`) 1)
      (if (or (`BlueprintSetLibrary.Set_IsEmpty` (`local.WinnerIDs`)) (== (`BlueprintSetLibrary.Set_Length` (`local.WinnerIDs`)) (`GameplayStatics.GetNumLocalPlayerControllers`)))
        ;[1 0.1406 0] Draw
        (if (`GameplayStatics.IsSplitscreenForceDisabled`)
          (bind _returnvalue (`|CreateWidget` "/Game/Core/Blueprints/UI/WBP_Result.WBP_Result_C" null -1))
          (`UserWidget.AddToViewport` _returnvalue 1)
          (return)
          (else
            (bind _controllerid (`/Game/Core/Blueprints/Libraries/BP_FestivalMacroLibrary.ForEachPlayer` (`GameplayStatics.GetGameMode`))
              (:`LoopBody`
                (bind _returnvalue_2 (`|CreateWidget` "/Game/Core/Blueprints/UI/WBP_Result.WBP_Result_C" (`GameplayStatics.GetPlayerControllerFromID` _controllerid) -1))
                (`UserWidget.AddToPlayerScreen` _returnvalue_2 1))
              (:`Completed`
                (return)))))
        (else
          ;[0 0.8828 1] Win or Lose
          (if (`GameplayStatics.IsSplitscreenForceDisabled`)
            (bind _result_2 (`BlueprintSetLibrary.Set_ToArray` (`local.WinnerIDs`)))
            (bind _returnvalue_3 (`|CreateWidget` "/Game/Core/Blueprints/UI/WBP_Result.WBP_Result_C" (`GameplayStatics.GetPlayerControllerFromID` (`|GetArrayItem` _result_2)) 1))
            (`UserWidget.AddToViewport` _returnvalue_3 1)
            (return)
            (else
              (bind _controllerid_2 (`/Game/Core/Blueprints/Libraries/BP_FestivalMacroLibrary.ForEachPlayer` (`GameplayStatics.GetGameMode`) :!label _label)
                (:`LoopBody`
                  (bind _returnvalue_4 (`|CreateWidget` "/Game/Core/Blueprints/UI/WBP_Result.WBP_Result_C" (`GameplayStatics.GetPlayerControllerFromID` _controllerid_2) (`KismetMathLibrary.Conv_BoolToInt` (`BlueprintSetLibrary.Set_Contains` (`local.WinnerIDs`) _controllerid_2))))
                  (`UserWidget.AddToPlayerScreen` _returnvalue_4 1))
                (:`Completed`
                  (return)))))))
      (else
        (goto _label)))))

(fn `ShowScore`
  (if (`KismetArrayLibrary.Array_IsEmpty` (`self.ScoreWidgets`))
    (if (`GameplayStatics.IsSplitscreenForceDisabled`)
      (bind _controllerid (`/Game/Core/Blueprints/Libraries/BP_FestivalMacroLibrary.ForEachPlayer` (`GameplayStatics.GetGameMode`))
        (:`LoopBody`
          (bind _returnvalue (`|CreateWidget` "/Game/Core/Blueprints/UI/WBP_Score.WBP_Score_C" (`GameplayStatics.GetPlayerControllerFromID` _controllerid)))
          (add `/Game/Core/Blueprints/UI/WBP_Score.OnScoreChanged` _returnvalue (`|CreateDelegate` :!event `CallOnScoreChanged`))
          (`KismetArrayLibrary.Array_Add` (`self.ScoreWidgets`) _returnvalue)
          (`UserWidget.AddToViewport` _returnvalue 1))
        (:`Completed`
          (return)))
      (else
        (bind _controllerid_2 (`/Game/Core/Blueprints/Libraries/BP_FestivalMacroLibrary.ForEachPlayer` (`GameplayStatics.GetGameMode`))
          (:`LoopBody`
            (bind _returnvalue_2 (`|CreateWidget` "/Game/Core/Blueprints/UI/WBP_Score.WBP_Score_C" (`GameplayStatics.GetPlayerControllerFromID` _controllerid_2)))
            (add `/Game/Core/Blueprints/UI/WBP_Score.OnScoreChanged` _returnvalue_2 (`|CreateDelegate` :!event `CallOnScoreChanged`))
            (`KismetArrayLibrary.Array_Add` (`self.ScoreWidgets`) _returnvalue_2)
            (`UserWidget.AddToPlayerScreen` _returnvalue_2 1))
          (:`Completed`
            (return)))))
    (else
      (`/Game/Core/Blueprints/UI/WBP_Score.ShowScore` (`self.ScoreWidgets`))
      (return))))

(fn `ShowTimer`
  (bind _timerwidget (`self.TimerWidget`)
    (:`then`
      (`/Game/Core/Blueprints/UI/WBP_Timer.ShowTimer` _timerwidget)
      (return))
    (:`else`
      (return))))

(fn `StartTimer`
  (bind _timerwidget (`self.TimerWidget`)
    (:`then`
      (`/Game/Core/Blueprints/UI/WBP_Timer.StartTimer` _timerwidget)
      (return))
    (:`else`
      (return))))

(fn `StopTimer`
  (bind _timerwidget (`self.TimerWidget`)
    (:`then`
      (`/Game/Core/Blueprints/UI/WBP_Timer.StopTimer` _timerwidget)
      (return))
    (:`else`
      (return))))

(fn `UserConstructionScript`)